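; Level exit actor that completes the level when the player first overlaps it, saving progress and playing the win effects.
; It stops the HUD timer, then marks its ExitIndex passed in the GameData save, adding a Thunder pass if elapsed time meets the spawner's requirement.
; It unlocks LevelsToUnlock through the cached save object, saving after each.
; Finally it spawns the win animation and disables the hidden amber ball.
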(event Collision|EventActorBeginOverlap
  (params (OtherActor :type Actor%20Object%20Reference))
  (bind _exitindex (Variables|Default|GetExitIndex))
  (bind _exitindex_2 (Variables|Default|GetExitIndex))
  (bind _asbp_player_character (Utilities|Casting|CastToBP_PlayerCharacter OtherActor))
  (if (not (Variables|Default|GetbOverlapOnce))
    (Variables|Default|SetbOverlapOnce true)
    (Utilities|FlowControl|Sequence
      (:then_0
        (bind _returnvalue (Actor|GetActorOfClass "/Game/Blueprints/MechanicsBPs/HUDSpawner/BP_HUDSpawner.BP_HUDSpawner_C"))
        (bind _output_get (Variables|Default|SetBP_HudSpawner _returnvalue))
        (bind _output_get_2 (Variables|Default|SetWBP%20Level%20Hud (Variables|/Game/Blueprints/MechanicsBPs/HUDSpawner/BP_HUDSpawner.BP_HUDSpawner_C|GetWBP%20Level%20Hud _output_get)))
        (Variables|/Game/Widgets/LevelHUD/WBP_LevelHUD.WBP_LevelHUD_C|SetbIsTimerRunning? _output_get_2 false))
      (:then_1
        (if (<= (Variables|/Game/Widgets/LevelHUD/WBP_LevelHUD.WBP_LevelHUD_C|GetElapsedTime (Variables|Default|GetWBP%20Level%20Hud)) (Variables|/Game/Blueprints/MechanicsBPs/HUDSpawner/BP_HUDSpawner.BP_HUDSpawner_C|GetThunderBadgeRequirement (Variables|Default|GetBP_HudSpawner)))
          (bind _asbp_game_data_save (CallFunction|LoadCastReturnGameDataSave))
          (Utilities|Array|SetArrayElem (Variables|/Game/Blueprints/SaveGameBPs/BP_GameDataSave.BP_GameDataSave_C|GetLevelProgressArray _asbp_game_data_save) _exitindex (Utilities|Struct|MakeBPS_LevelProgress (.levelid (Utilities|Array|Get(acopy) (Variables|/Game/Blueprints/SaveGameBPs/BP_GameDataSave.BP_GameDataSave_C|GetLevelProgressArray _asbp_game_data_save) _exitindex)) (.bunlocked (Utilities|Array|Get(acopy) (Variables|/Game/Blueprints/SaveGameBPs/BP_GameDataSave.BP_GameDataSave_C|GetLevelProgressArray _asbp_game_data_save) _exitindex)) true (.bacepassed (Utilities|Array|Get(acopy) (Variables|/Game/Blueprints/SaveGameBPs/BP_GameDataSave.BP_GameDataSave_C|GetLevelProgressArray _asbp_game_data_save) _exitindex)) true))
          (SaveGame|SaveGametoSlot _asbp_game_data_save "GameData")
          (Development|PrintString (Utilities|String|Append "This Exit index is" (Utilities|String|ToString(Integer) _exitindex) "retrieved level id was" (Utilities|String|ToString(Integer) (.levelid (Utilities|Array|Get(acopy) (Variables|/Game/Blueprints/SaveGameBPs/BP_GameDataSave.BP_GameDataSave_C|GetLevelProgressArray _asbp_game_data_save) _exitindex))) "level saved as thunder passed"))
          (else
            (bind _asbp_game_data_save_2 (CallFunction|LoadCastReturnGameDataSave))
            (Utilities|Array|SetArrayElem (Variables|/Game/Blueprints/SaveGameBPs/BP_GameDataSave.BP_GameDataSave_C|GetLevelProgressArray _asbp_game_data_save_2) _exitindex_2 (Utilities|Struct|MakeBPS_LevelProgress (.levelid (Utilities|Array|Get(acopy) (Variables|/Game/Blueprints/SaveGameBPs/BP_GameDataSave.BP_GameDataSave_C|GetLevelProgressArray _asbp_game_data_save_2) _exitindex_2)) (.bunlocked (Utilities|Array|Get(acopy) (Variables|/Game/Blueprints/SaveGameBPs/BP_GameDataSave.BP_GameDataSave_C|GetLevelProgressArray _asbp_game_data_save_2) _exitindex_2)) true (.bacepassed (Utilities|Array|Get(acopy) (Variables|/Game/Blueprints/SaveGameBPs/BP_GameDataSave.BP_GameDataSave_C|GetLevelProgressArray _asbp_game_data_save_2) _exitindex_2)) (.bthunderpassed (Utilities|Array|Get(acopy) (Variables|/Game/Blueprints/SaveGameBPs/BP_GameDataSave.BP_GameDataSave_C|GetLevelProgressArray _asbp_game_data_save_2) _exitindex_2))))
            (SaveGame|SaveGametoSlot _asbp_game_data_save_2 "GameData")
            (Development|PrintString (Utilities|String|Append "This Exit index is" (Utilities|String|ToString(Integer) _exitindex_2) "retrieved level id was" (Utilities|String|ToString(Integer) (.levelid (Utilities|Array|Get(acopy) (Variables|/Game/Blueprints/SaveGameBPs/BP_GameDataSave.BP_GameDataSave_C|GetLevelProgressArray _asbp_game_data_save_2) _exitindex_2))) "level saved as normal passed")))))
      (:then_2
        (CallFunction|UnlockLevelsThenSaveGame (Variables|Default|GetLevelsToUnlock)))
      (:then_3
        (Audio|PlaySound2D "/Game/Sound/GameMechanics/SFX00_Win.SFX00_Win" 1.0 1.0 0.0 0 0 :!label _label)
        (Game|SpawnActorfromClass "/Game/Characters/CH01_AmberBall/BP_PlayerWinAnimation.BP_PlayerWinAnimation_C" (Math|Conversions|ToTransform(Vector) (Transformation|GetWorldLocation (Variables|/Game/Characters/CH01_AmberBall/BP_PlayerCharacter.BP_PlayerCharacter_C|GetSM_AmberBall _asbp_player_character))) "Undefined" 0 0)
        (Development|SetHiddeninGame (Variables|/Game/Characters/CH01_AmberBall/BP_PlayerCharacter.BP_PlayerCharacter_C|GetSM_AmberBall _asbp_player_character) true true)
        (Collision|SetCollisionResponsetoAllChannels (Variables|/Game/Characters/CH01_AmberBall/BP_PlayerCharacter.BP_PlayerCharacter_C|GetSM_AmberBall _asbp_player_character) "ECR_Ignore")
        (Physics|SetSimulatePhysics (Variables|/Game/Characters/CH01_AmberBall/BP_PlayerCharacter.BP_PlayerCharacter_C|GetSM_AmberBall _asbp_player_character) false)
        (Variables|/Game/Characters/CH01_AmberBall/BP_PlayerCharacter.BP_PlayerCharacter_C|SetbHasPassed _asbp_player_character true))
      (:then_4
        (goto _label)))))

(fn ConstructionScript)

(fn UnlockLevelsThenSaveGame
  (params (LevelsToUnlock :type Array%20of%20Integers))
  (bind _bp_gamedatasave (Variables|Default|GetBP_GameDataSave))
  (bind _levelprogressarray (Variables|/Game/Blueprints/SaveGameBPs/BP_GameDataSave.BP_GameDataSave_C|GetLevelProgressArray _bp_gamedatasave))
  (for _array_element LevelsToUnlock
    (Utilities|Array|SetArrayElem _levelprogressarray _array_element (Utilities|Struct|MakeBPS_LevelProgress (.LevelID (Utilities|Struct|BreakBPS_LevelProgress (Utilities|Array|Get(acopy) _levelprogressarray _array_element))) true (.bPassed (Utilities|Struct|BreakBPS_LevelProgress (Utilities|Array|Get(acopy) _levelprogressarray _array_element))) (.bAcePassed (Utilities|Struct|BreakBPS_LevelProgress (Utilities|Array|Get(acopy) _levelprogressarray _array_element))) (.bThunderPassed (Utilities|Struct|BreakBPS_LevelProgress (Utilities|Array|Get(acopy) _levelprogressarray _array_element)))))
    (SaveGame|SaveGametoSlot _bp_gamedatasave "GameData")
    (Development|PrintString (Utilities|String|Append "Level" (Utilities|String|ToString(Integer) (.LevelID (Utilities|Struct|BreakBPS_LevelProgress (Utilities|Array|Get(acopy) _levelprogressarray _array_element)))) "was unlocked!") true true "(R=0.231290,G=1.000000,B=0.000000,A=1.000000)")))

(fn LoadCastReturnGameDataSave
  (bind _returnvalue (SaveGame|LoadGamefromSlot "GameData"))
  (bind _asbp_game_data_save (Utilities|Casting|CastToBP_GameDataSave _returnvalue))
  (bind _output_get (Variables|Default|SetBP_GameDataSave _asbp_game_data_save))
  (return _output_get))