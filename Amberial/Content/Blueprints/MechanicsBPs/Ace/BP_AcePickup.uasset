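; BP_AcePickup is a per-level Ace collectible that records its pickup in the GameData save slot.
; BeginPlay reads that level's AcePassed flag, dims the dynamic icon and square materials if already collected, and starts timelines animating tint and scale while Tick spins the square.
; The first overlap by any actor sets the flag, increments and saves AceAmount, plays a sound, dims the meshes and spawns BP_AceAnim.
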(event EventBeginPlay
  (Utilities|FlowControl|Sequence
    (:then_0
      (bind _gamedatasave (CallFunction|LoadCastReturnGameDataSave))
      (if (.bAcePassed (Utilities|Struct|BreakBPS_LevelProgress (Utilities|Array|Get(acopy) (Variables|/Game/Blueprints/SaveGameBPs/BP_GameDataSave.BP_GameDataSave_C|GetLevelProgressArray _gamedatasave) (Variables|Default|GetLevelIndex))))
        (Variables|Default|SetbIsAcePicked true)
        (else
          (Variables|Default|SetbIsAcePicked false)))
      (Development|PrintString (Utilities|String|Append "Level:" (Utilities|String|ToString(Integer) (.LevelID (Utilities|Struct|BreakBPS_LevelProgress (Utilities|Array|Get(acopy) (Variables|/Game/Blueprints/SaveGameBPs/BP_GameDataSave.BP_GameDataSave_C|GetLevelProgressArray _gamedatasave) (Variables|Default|GetLevelIndex))))) "Ace Passed:" (Utilities|String|ToString(Boolean) (.bAcePassed (Utilities|Struct|BreakBPS_LevelProgress (Utilities|Array|Get(acopy) (Variables|/Game/Blueprints/SaveGameBPs/BP_GameDataSave.BP_GameDataSave_C|GetLevelProgressArray _gamedatasave) (Variables|Default|GetLevelIndex))))))))
    (:then_1
      (bind _returnvalue (Rendering|Material|CreateDynamicMaterialInstance (Variables|Default|GetSM_AceIcon) 0 "/Game/Blueprints/MechanicsBPs/Ace/M_AceIcon.M_AceIcon" "None" :!class /Script/Engine.PrimitiveComponent))
      (Variables|Default|SetMI_AceIcon _returnvalue)
      (bind _returnvalue_2 (Rendering|Material|CreateDynamicMaterialInstance (Variables|Default|GetSM_AceSquare) 0 "/Game/Blueprints/MechanicsBPs/Ace/M_AceSquare.M_AceSquare" "None" :!class /Script/Engine.PrimitiveComponent))
      (Variables|Default|SetMI_AceSquare _returnvalue_2))
    (:then_2
      (if (Variables|Default|GetbIsAcePicked)
        (Rendering|Material|SetScalarParameterValue (Variables|Default|GetMI_AceSquare) "Opacity" 0.1 :!class /Script/Engine.MaterialInstanceDynamic)
        (Rendering|Material|SetScalarParameterValue (Variables|Default|GetMI_AceIcon) "Opacity" 0.1 :!class /Script/Engine.MaterialInstanceDynamic)))
    (:then_3
      (bind _newtrack_0 (Timeline|AceColorAnim PlayFromStart)
        (:Update
          (Rendering|Material|SetVectorParameterValue (Variables|Default|GetMI_AceIcon) "Tint" _newtrack_0 :!class /Script/Engine.MaterialInstanceDynamic)
          (Rendering|Material|SetVectorParameterValue (Variables|Default|GetMI_AceSquare) "Tint" _newtrack_0 :!class /Script/Engine.MaterialInstanceDynamic)
          (bind _newtrack_0_2 (Timeline|ScaleAnim Play)
            (:Update
              (Transformation|SetRelativeScale3D (Variables|Default|GetSM_AceSquare) (Math|Conversions|ToVector(Float) _newtrack_0_2))
              (Transformation|SetRelativeScale3D (Variables|Default|GetSM_AceIcon) (Math|Conversions|ToVector(Float) _newtrack_0_2)))))))))

(event Collision|EventActorBeginOverlap
  (params (OtherActor :type Actor%20Object%20Reference))
  (bind _levelindex (Variables|Default|GetLevelIndex))
  (if (not (Variables|Default|GetbIsAcePicked))
    (Utilities|FlowControl|Sequence
      (:then_0
        (Variables|Default|SetbIsAcePicked true)
        (bind _gamedatasave (CallFunction|LoadCastReturnGameDataSave))
        (Utilities|Array|SetArrayElem (Variables|/Game/Blueprints/SaveGameBPs/BP_GameDataSave.BP_GameDataSave_C|GetLevelProgressArray _gamedatasave) _levelindex (Utilities|Struct|MakeBPS_LevelProgress (.LevelID (Utilities|Struct|BreakBPS_LevelProgress (Utilities|Array|Get(acopy) (Variables|/Game/Blueprints/SaveGameBPs/BP_GameDataSave.BP_GameDataSave_C|GetLevelProgressArray _gamedatasave) _levelindex))) (.bUnlocked (Utilities|Struct|BreakBPS_LevelProgress (Utilities|Array|Get(acopy) (Variables|/Game/Blueprints/SaveGameBPs/BP_GameDataSave.BP_GameDataSave_C|GetLevelProgressArray _gamedatasave) _levelindex))) (.bPassed (Utilities|Struct|BreakBPS_LevelProgress (Utilities|Array|Get(acopy) (Variables|/Game/Blueprints/SaveGameBPs/BP_GameDataSave.BP_GameDataSave_C|GetLevelProgressArray _gamedatasave) _levelindex))) true))
        (bind _output_get (Variables|/Game/Blueprints/SaveGameBPs/BP_GameDataSave.BP_GameDataSave_C|SetAceAmount _gamedatasave (+ (Variables|/Game/Blueprints/SaveGameBPs/BP_GameDataSave.BP_GameDataSave_C|GetAceAmount _gamedatasave) 1)))
        (SaveGame|SaveGametoSlot _gamedatasave "GameData")
        (Development|PrintString (Utilities|String|Append "Ace Amount is now:" (Utilities|String|ToString(Integer) _output_get))))
      (:then_2
        (Audio|PlaySound2D "/Game/Sound/GameMechanics/SFX01_Ace.SFX01_Ace" 1.0 1.0 0.0 0 0))
      (:then_3
        (Rendering|Material|SetScalarParameterValue (Variables|Default|GetMI_AceSquare) "Opacity" 0.1 :!class /Script/Engine.MaterialInstanceDynamic)
        (Rendering|Material|SetScalarParameterValue (Variables|Default|GetMI_AceIcon) "Opacity" 0.1 :!class /Script/Engine.MaterialInstanceDynamic))
      (:then_4
        (Game|SpawnActorfromClass "/Game/Blueprints/MechanicsBPs/Ace/BP_AceAnim.BP_AceAnim_C" (Math|Transform|MakeTransform (Transformation|GetActorLocation) "0, 0, 0" (Transformation|GetWorldScale (Variables|Default|GetDefaultSceneRoot))) "Undefined" 0 0)))))

(event EventTick
  (params (DeltaSeconds :type Float%20%28single-precision%29))
  (Transformation|AddRelativeRotation (Variables|Default|GetSM_AceSquare) (Math|Rotator|MakeRotator (* DeltaSeconds -4e+02) 0.0 0.0) false false))

(fn ConstructionScript
  (Utilities|FlowControl|Sequence))

(fn LoadCastReturnGameDataSave
  (bind _returnvalue (SaveGame|LoadGamefromSlot "GameData"))
  (bind _asbp_game_data_save (Utilities|Casting|CastToBP_GameDataSave _returnvalue))
  (return _asbp_game_data_save))