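; BP_AceAnim is a short-lived effect actor that animates an Ace icon and square, apparently as feedback for getting an ace.
; Its construction script creates dynamic material instances for both meshes, which BeginPlay tints orange.
; A timeline scales both meshes while triggering a second timeline that drives their opacity.
; The actor destroys itself when the scale timeline finishes.
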(event EventBeginPlay
  (Rendering|Material|SetVectorParameterValue (Variables|Default|GetMI_AceIcon) "Tint" "(R=1.000000,G=0.456411,B=0.000000,A=1.000000)" :!class /Script/Engine.MaterialInstanceDynamic)
  (Rendering|Material|SetVectorParameterValue (Variables|Default|GetMI_AceSquare) "Tint" "(R=1.000000,G=0.456411,B=0.000000,A=1.000000)" :!class /Script/Engine.MaterialInstanceDynamic)
  (bind _newtrack_0 (Timeline|AceGetScaleUP PlayFromStart)
    (:Update
      (Transformation|SetRelativeScale3D (Variables|Default|GetSM_AceSquare) (Math|Conversions|ToVector(Float) _newtrack_0))
      (Transformation|SetRelativeScale3D (Variables|Default|GetSM_AceIcon) (Math|Conversions|ToVector(Float) _newtrack_0))
      (bind _newtrack_0_2 (Timeline|OpacityAnim Play)
        (:Update
          (Rendering|Material|SetScalarParameterValue (Variables|Default|GetMI_AceSquare) "Opacity" _newtrack_0_2 :!class /Script/Engine.MaterialInstanceDynamic)
          (Rendering|Material|SetScalarParameterValue (Variables|Default|GetMI_AceIcon) "Opacity" _newtrack_0_2 :!class /Script/Engine.MaterialInstanceDynamic))))
    (:Finished
      (Actor|DestroyActor))))

(fn ConstructionScript
  (Utilities|FlowControl|Sequence
    (:then_0
      (bind _returnvalue (Rendering|Material|CreateDynamicMaterialInstance (Variables|Default|GetSM_AceIcon) 0 "/Game/Blueprints/MechanicsBPs/Ace/M_AceIcon.M_AceIcon" "None" :!class /Script/Engine.PrimitiveComponent))
      (Variables|Default|SetMI_AceIcon _returnvalue)
      (bind _returnvalue_2 (Rendering|Material|CreateDynamicMaterialInstance (Variables|Default|GetSM_AceSquare) 0 "/Game/Blueprints/MechanicsBPs/Ace/M_AceSquare.M_AceSquare" "None" :!class /Script/Engine.PrimitiveComponent))
      (Variables|Default|SetMI_AceSquare _returnvalue_2))))