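; BP_FollowCamera is a camera actor that becomes the player's view and follows the BP_PlayerCharacter.
; On BeginPlay it sets itself as the first player controller's view target, then attaches to the character, snapping to its location while keeping relative rotation and scale.
; A ZoomOutAnim timeline that would move the Camera along local X is present, but nothing starts it.
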(event EventBeginPlay
  (CallFunction|BlendtoCamera)
  (bind _returnvalue (Actor|GetActorOfClass "/Game/Characters/CH01_AmberBall/BP_PlayerCharacter.BP_PlayerCharacter_C"))
  (Transformation|AttachActorToActor self _returnvalue "None" "SnapToTarget" "KeepRelative" "KeepRelative" false))

(fn ConstructionScript)

(fn BlendtoCamera
  (Game|Player|SetViewTargetwithBlend (Game|GetPlayerController 0) self 0.0 "VTBlend_Linear" 0.0 false))