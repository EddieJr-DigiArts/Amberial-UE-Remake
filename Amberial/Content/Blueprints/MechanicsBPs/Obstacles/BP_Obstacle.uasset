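; BP_Obstacle is a lava hazard that kills the player on contact.
; On BeginPlay, the ScaleZUP timeline animates the LavaCube's Z scale as an offset from its original value.
; When BP_PlayerCharacter overlaps it, it plays a death sound and clears IsAlive.
; It then hides the amber ball, disables its collision response, physics and the player's tick, and spawns BP_PlayerDeathAnim at the ball's location.
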(event EventBeginPlay
  (bind _lavacube (Variables|Default|GetLavaCube))
  (bind _returnvalue (Transformation|GetWorldScale _lavacube))
  (Variables|Default|SetOriginalZScale (.z (Transformation|GetWorldScale (Variables|Default|GetLavaCube))))
  (bind _newtrack_0 (Timeline|ScaleZUP Play)
    (:Update
      (Transformation|SetWorldScale3D _lavacube (Math|Vector|MakeVector (.x _returnvalue) (.y _returnvalue) (+ (Variables|Default|GetOriginalZScale) _newtrack_0))))))

(event Collision|EventActorBeginOverlap
  (params (OtherActor :type Actor%20Object%20Reference))
  (bind _asbp_player_character (Utilities|Casting|CastToBP_PlayerCharacter OtherActor))
  (Utilities|FlowControl|Sequence
    (:then_0
      (Audio|PlaySound2D "/Game/Sound/CharactersSounds/CHSFX04_Death.CHSFX04_Death" 1.0 1.0 0.0 0 0))
    (:then_1
      (Variables|/Game/Characters/CH01_AmberBall/BP_PlayerCharacter.BP_PlayerCharacter_C|SetbIsAlive _asbp_player_character false))
    (:then_2
      (Development|SetHiddeninGame (Variables|/Game/Characters/CH01_AmberBall/BP_PlayerCharacter.BP_PlayerCharacter_C|GetSM_AmberBall _asbp_player_character) true true)
      (Collision|SetCollisionResponsetoAllChannels (Variables|/Game/Characters/CH01_AmberBall/BP_PlayerCharacter.BP_PlayerCharacter_C|GetSM_AmberBall _asbp_player_character) "ECR_Ignore")
      (Physics|SetSimulatePhysics (Variables|/Game/Characters/CH01_AmberBall/BP_PlayerCharacter.BP_PlayerCharacter_C|GetSM_AmberBall _asbp_player_character) false)
      (Actor|Tick|SetActorTickEnabled _asbp_player_character))
    (:then_3
      (Game|SpawnActorfromClass "/Game/Characters/CH01_AmberBall/BP_PlayerDeathAnim.BP_PlayerDeathAnim_C" (Math|Conversions|ToTransform(Vector) (Transformation|GetWorldLocation (Variables|/Game/Characters/CH01_AmberBall/BP_PlayerCharacter.BP_PlayerCharacter_C|GetSM_AmberBall _asbp_player_character))) "Undefined" 0 0))))

(fn ConstructionScript)