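; BP_RimLightManager is an unfinished manager meant to apply rim-light color to meshes across the level.
; On BeginPlay it scans every actor's static and skeletal mesh components.
; Static meshes go to SetStaticMeshRimlightColor, which creates and prints dynamic instances of their material instances, without assigning them or setting any color.
; Skeletal meshes only have their names printed.
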(event EventBeginPlay
  (bind _outactors (Actor|GetAllActorsOfClass "/Script/Engine.Actor"))
  (for _array_element _outactors
    (for _array_element_2 (Actor|GetComponentsByClass _array_element "/Script/Engine.StaticMeshComponent")
      (CallFunction|SetStaticMeshRimlightColor _array_element_2))
    (for _array_element_3 (Actor|GetComponentsByClass _array_element "/Script/Engine.SkeletalMeshComponent")
      (Development|PrintString (Utilities|GetDisplayName _array_element_3)))))

(event Collision|EventActorBeginOverlap
  (params (OtherActor :type Actor%20Object%20Reference)))

(event EventTick
  (params (DeltaSeconds :type Float%20%28single-precision%29)))

(fn ConstructionScript)

(fn SetStaticMeshRimlightColor
  (params (StaticMesh :type Static%20Mesh%20Component%20Object%20Reference))
  (for _array_element (Rendering|Material|GetMaterials StaticMesh)
    (bind _asmaterial_instance (Utilities|Casting|CastToMaterialInstance _array_element))
    (bind _returnvalue (Rendering|Material|CreateDynamicMaterialInstance _asmaterial_instance "None" "None" :!class /Script/Engine.KismetMaterialLibrary))
    (Development|PrintString (Utilities|GetDisplayName _returnvalue))))