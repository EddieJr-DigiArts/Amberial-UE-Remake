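; Spring pad that compresses when hit by the player and launches their amber ball with a vertical impulse.
; A hit plays a timeline that moves the mesh and ball along Z and animates the bottom light's emissive, then fires the impulse if the player remains on it.
; When Cumulative is set, hit force scales travel and launch strength.
; Top and bottom triggers track the rider and switch collision, letting the ball pass through from below.
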(event OnComponentBeginOverlap(BottomCollision)
  (params (OverlappedComponent :type Primitive%20Component%20Object%20Reference) (OtherActor :type Actor%20Object%20Reference) (OtherComp :type Primitive%20Component%20Object%20Reference) (OtherBodyIndex :type Integer) (bFromSweep :type Boolean) (SweepResult :type Hit%20Result%20Structure%20%28by%20ref%29))
  (Utilities|Casting|CastToBP_PlayerCharacter OtherActor)
  (Collision|SetCollisionResponsetoAllChannels (Variables|Default|GetSpringMesh) "ECR_Ignore")
  (Collision|SetCollisionResponsetoAllChannels (Variables|Default|GetTopCollision) "ECR_Ignore")
  (Development|PrintString "Ball came from below, turn off collision"))

(event OnComponentEndOverlap(BottomCollision)
  (params (OverlappedComponent :type Primitive%20Component%20Object%20Reference) (OtherActor :type Actor%20Object%20Reference) (OtherComp :type Primitive%20Component%20Object%20Reference) (OtherBodyIndex :type Integer))
  (Utilities|Casting|CastToBP_PlayerCharacter OtherActor)
  (Collision|SetCollisionResponsetoAllChannels (Variables|Default|GetSpringMesh) "ECR_Block")
  (Collision|SetCollisionResponsetoAllChannels (Variables|Default|GetTopCollision) "ECR_Overlap"))

(event OnComponentBeginOverlap(TopCollision)
  (params (OverlappedComponent :type Primitive%20Component%20Object%20Reference) (OtherActor :type Actor%20Object%20Reference) (OtherComp :type Primitive%20Component%20Object%20Reference) (OtherBodyIndex :type Integer) (bFromSweep :type Boolean) (SweepResult :type Hit%20Result%20Structure%20%28by%20ref%29))
  (Utilities|Casting|CastToBP_PlayerCharacter OtherActor)
  (Variables|Default|SetbIsPlayerOnSpring true)
  (Collision|SetCollisionResponsetoAllChannels (Variables|Default|GetBottomCollision) "ECR_Ignore"))

(event OnComponentEndOverlap(TopCollision)
  (params (OverlappedComponent :type Primitive%20Component%20Object%20Reference) (OtherActor :type Actor%20Object%20Reference) (OtherComp :type Primitive%20Component%20Object%20Reference) (OtherBodyIndex :type Integer))
  (Utilities|Casting|CastToBP_PlayerCharacter OtherActor)
  (Variables|Default|SetbIsPlayerOnSpring false))

(event OnComponentHit(SpringMesh)
  (params (HitComponent :type Primitive%20Component%20Object%20Reference) (OtherActor :type Actor%20Object%20Reference) (OtherComp :type Primitive%20Component%20Object%20Reference) (NormalImpulse :type Vector :default "0, 0, 0") (Hit :type Hit%20Result%20Structure%20%28by%20ref%29))
  (bind _returnvalue (Math|Float|MapRangeClamped (.z NormalImpulse) 0.0 4e+05 1.0 3.0))
  (bind _sm_amberballref (Variables|Default|GetSM_AmberBallRef))
  (bind _fzlocationoriginal (Variables|Default|GetfZLocationOriginal))
  (bind _springmesh (Variables|Default|GetSpringMesh))
  (bind _returnvalue_2 (Transformation|GetWorldLocation _springmesh))
  (bind _returnvalue_3 (Transformation|GetWorldLocation _sm_amberballref))
  (if (not (Variables|Default|GetbOverlapOnce))
    (Variables|Default|SetbOverlapOnce true)
    (Development|PrintString (Utilities|String|ToString(Float) _returnvalue))
    (Utilities|Casting|CastToBP_PlayerCharacter OtherActor)
    (Variables|Default|SetbIsPlayerOnSpring true)
    (Utilities|FlowControl|Sequence
      (:then_0
        (if (Variables|Default|GetbCumulative)
          (Variables|Default|SetfZImpulseMultiplier _returnvalue)))
      (:then_1
        (if (not (Variables|Default|GetbIsSpringMoving))
          (Audio|PlaySoundatLocation "/Game/Sound/GameMechanics/SFX04_SpringDown.SFX04_SpringDown" (Transformation|GetWorldLocation (Variables|Default|GetSpringMesh)) "0, 0, 0" 1.0 1.0 0.0 0 0 0)
          (Components|Timeline|SetPlayRate (Variables|Default|GetTL_SpringAnim) (Variables|Default|GetfCompressionSpeed))
          (bind (_direction _springzanimation _emissivestrength) (Timeline|TL_SpringAnim PlayFromStart)
            (:Update
              (Variables|Default|SetbIsSpringMoving true)
              (Transformation|SetWorldLocation (Variables|Default|GetSpringMesh) (Math|Vector|MakeVector (.x _returnvalue_2) (.y _returnvalue_2) (Math|Float|Lerp _fzlocationoriginal (+ _fzlocationoriginal (* (Variables|Default|GetfZLocationTarget) (Variables|Default|GetfZImpulseMultiplier))) _springzanimation)) false true)
              (Rendering|Material|SetScalarParameterValue (Variables|Default|GetMI_SpringBottomLight) "EmissiveStrength" _emissivestrength :!class /Script/Engine.MaterialInstanceDynamic)
              (if (Variables|Default|GetbIsPlayerOnSpring)
                (Transformation|SetWorldLocation _sm_amberballref (Math|Vector|MakeVector (.x _returnvalue_3) (.y _returnvalue_3) (+ (Math|Float|Lerp _fzlocationoriginal (+ _fzlocationoriginal (* (Variables|Default|GetfZLocationTarget) (Variables|Default|GetfZImpulseMultiplier))) _springzanimation) 8e+01)) false true)
                (Collision|SetCollisionResponsetoAllChannels (Variables|Default|GetBottomCollision) "ECR_Ignore")))
            (:Finished
              (Audio|PlaySoundatLocation "/Game/Sound/GameMechanics/SFX03_SpringUP.SFX03_SpringUP" (Transformation|GetWorldLocation (Variables|Default|GetSpringMesh)) "0, 0, 0" 1.0 1.0 0.0 0 0 0)
              (Rendering|Material|SetScalarParameterValue (Variables|Default|GetMI_SpringBottomLight) "EmissiveStrength" 0.0 :!class /Script/Engine.MaterialInstanceDynamic)
              (Variables|Default|SetbIsSpringMoving false)
              (Variables|Default|SetbOverlapOnce false)
              (if (Variables|Default|GetbIsPlayerOnSpring)
                (Physics|AddImpulse (Variables|Default|GetSM_AmberBallRef) (Math|Vector|MakeVector 0.0 0.0 (* (Variables|Default|GetfZImpulseBase) (Variables|Default|GetfZImpulseMultiplier))) "None" true)
                (Variables|Default|SetbIsPlayerOnSpring false)))))))))

(event EventBeginPlay
  (bind _springmesh (Variables|Default|GetSpringMesh))
  (Utilities|FlowControl|Sequence
    (:then_0
      (bind _returnvalue (Rendering|Material|CreateDynamicMaterialInstance _springmesh 4 (Rendering|Material|GetMaterial _springmesh 4) "None" :!class /Script/Engine.PrimitiveComponent))
      (Variables|Default|SetMI_SpringBottomLight _returnvalue)
      (Variables|Default|SetfZLocationOriginal (.z (Transformation|GetWorldLocation (Variables|Default|GetSpringMesh)))))
    (:then_1
      (bind _returnvalue_2 (Actor|GetActorOfClass "/Game/Characters/CH01_AmberBall/BP_PlayerCharacter.BP_PlayerCharacter_C"))
      (bind _output_get (Variables|Default|SetBP_PlayerCharacterRef _returnvalue_2))
      (Variables|Default|SetSM_AmberBallRef (Variables|/Game/Characters/CH01_AmberBall/BP_PlayerCharacter.BP_PlayerCharacter_C|GetSM_AmberBall _output_get)))))

(fn ConstructionScript)