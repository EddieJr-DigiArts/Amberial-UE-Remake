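; Game instance Blueprint that sets up save slots and restores user audio and display settings at startup.
; On Init it asynchronously creates the UserSettings and GameData saves if either is missing.
; It then async-loads UserSettings to apply SFX and BGM volumes through sound mix overrides, plus window mode and scalability through GameUserSettings.
; The loads do not wait for save creation to finish, and debug prints report each step.
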(event EventInit
  (Utilities|FlowControl|Sequence
    (:then_0
      ;[0 0.1092 0.15 0.5] Create UserSettings Save
      (bind _returnvalue (SaveGame|DoesSaveGameExist "UserSettings"))
      (if (not _returnvalue)
        (bind _returnvalue_2 (SaveGame|CreateSaveGameObject "/Game/Blueprints/SaveGameBPs/BP_UserSettingsSave.BP_UserSettingsSave_C"))
        (|AsyncSaveGametoSlot _returnvalue_2 "UserSettings"
          (:Completed
            (Development|PrintString "CreatedUserSettings")))))
    (:then_1
      ;[0.03807 0.003903 0.15 0.5] Create GameData Save
      (bind _returnvalue_3 (SaveGame|DoesSaveGameExist "GameData"))
      (if (not _returnvalue_3)
        (bind _returnvalue_4 (SaveGame|CreateSaveGameObject "/Game/Blueprints/SaveGameBPs/BP_GameDataSave.BP_GameDataSave_C"))
        (|AsyncSaveGametoSlot _returnvalue_4 "GameData"
          (:Completed
            (Development|PrintString "CreateGameDataSave")))))
    (:then_2
      ;[0.15 1.8e-05 0.004755 0.5] Restore Sound Settings
      (bind _savegame (|AsyncLoadGamefromSlot "UserSettings")
        (:Completed
          (bind _asbp_user_settings_save (Utilities|Casting|CastToBP_UserSettingsSave _savegame))
          (Audio|SetSoundMixClassOverride "/Game/Sound/SCM_SFX.SCM_SFX" "/Game/Sound/SC_SFX.SC_SFX" (Variables|/Game/Blueprints/SaveGameBPs/BP_UserSettingsSave.BP_UserSettingsSave_C|GetSFXVolumeSave _asbp_user_settings_save) 1.0 0.0 true)
          (Audio|PushSoundMixModifier "/Game/Sound/SCM_SFX.SCM_SFX")
          (Audio|SetSoundMixClassOverride "/Game/Sound/SCM_BGM.SCM_BGM" "/Game/Sound/SC_BGM.SC_BGM" (Variables|/Game/Blueprints/SaveGameBPs/BP_UserSettingsSave.BP_UserSettingsSave_C|GetBGMVolumeSave _asbp_user_settings_save) 1.0 0.0 true)
          (Audio|PushSoundMixModifier "/Game/Sound/SCM_BGM.SCM_BGM")
          (Development|PrintString "Restored Audio Settings" true true "(R=0.230516,G=1.000000,B=0.000000,A=1.000000)" 5.0)
          (Development|PrintString (Utilities|String|ToString(Float) (Variables|/Game/Blueprints/SaveGameBPs/BP_UserSettingsSave.BP_UserSettingsSave_C|GetSFXVolumeSave _asbp_user_settings_save)) true true "(R=0.375404,G=1.000000,B=0.000000,A=1.000000)" 5.0)
          (Development|PrintString (Utilities|String|ToString(Float) (Variables|/Game/Blueprints/SaveGameBPs/BP_UserSettingsSave.BP_UserSettingsSave_C|GetBGMVolumeSave _asbp_user_settings_save)) true true "(R=0.495538,G=1.000000,B=0.000000,A=1.000000)" 5.0))))
    (:then_3
      ;[0.15 0.07568 0 0.5] Restore Display Settings
      (bind _savegame_2 (|AsyncLoadGamefromSlot "UserSettings")
        (:Completed
          (bind _asbp_user_settings_save_2 (Utilities|Casting|CastToBP_UserSettingsSave _savegame_2))
          (bind _returnvalue_5 (Settings|GetGameUserSettings))
          (Class|GameUserSettings|SetFullscreenMode _returnvalue_5 (Variables|/Game/Blueprints/SaveGameBPs/BP_UserSettingsSave.BP_UserSettingsSave_C|GetWindowModeSave _asbp_user_settings_save_2))
          (Class|GameUserSettings|SetOverallScalabilityLevel _returnvalue_5 (Variables|/Game/Blueprints/SaveGameBPs/BP_UserSettingsSave.BP_UserSettingsSave_C|GetScalabilityLevelSave _asbp_user_settings_save_2))
          (Class|GameUserSettings|ApplySettings _returnvalue_5 false)
          (Development|PrintString "Restored Display Settings With" true true "(R=0.000000,G=0.258183,B=1.000000,A=1.000000)" 5.0)
          (Development|PrintString (Utilities|String|EnumtoString (Variables|/Game/Blueprints/SaveGameBPs/BP_UserSettingsSave.BP_UserSettingsSave_C|GetWindowModeSave _asbp_user_settings_save_2)) true true "(R=0.000000,G=0.181620,B=1.000000,A=1.000000)" 5.0)
          (Development|PrintString (Utilities|String|ToString(Integer) (Variables|/Game/Blueprints/SaveGameBPs/BP_UserSettingsSave.BP_UserSettingsSave_C|GetScalabilityLevelSave _asbp_user_settings_save_2)) true true "(R=0.000000,G=0.293773,B=1.000000,A=1.000000)" 5.0))))))