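; Player character for the amber ball, a physics-driven ball steered sideways by axis input as force, with Tick clamping its lateral velocity.
; BeginPlay blends the camera to it and plays a scale-up timeline, whose update also sets a looping trail timer and binds the hit event.
; Niagara trails spawn while it is alive and has not passed.
; Hits on "HittablePlatform" actors play cooldown-limited sounds chosen by vertical speed.
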(event Custom|OnComponentHit_Event_0
  (params (HitComponent :type Primitive%20Component%20Object%20Reference) (OtherActor :type Actor%20Object%20Reference) (OtherComp :type Primitive%20Component%20Object%20Reference) (NormalImpulse :type Vector) (Hit :type Hit%20Result%20Structure%20%28by%20ref%29))
  (if (Actor|ActorHasTag OtherActor "HittablePlatform")
    (if (>= (- (Utilities|Time|GetGameTimeinSeconds) (Variables|Default|GetfLastHitSound)) (Variables|Default|GetfHitSoundCooldown))
      (CallFunction|HitSoundPitchManager)
      (Variables|Default|SetfLastHitSound (Utilities|Time|GetGameTimeinSeconds)))))

(event EventTick
  (params (DeltaSeconds :type Float%20%28single-precision%29))
  (Utilities|FlowControl|Sequence
    (:then_0
      ;[0 0.458 1] Clamp Y Velocity
      (bind _returnvalue (Physics|GetPhysicsLinearVelocity (Variables|Default|GetSM_AmberBall) "None"))
      (if (>= (Math|Float|Absolute(Float) (.Y (Math|Vector|BreakVector _returnvalue))) 5e+02)
        (Physics|SetPhysicsLinearVelocity (Variables|Default|GetSM_AmberBall) (Math|Vector|MakeVector (.X (Math|Vector|BreakVector _returnvalue)) (Math|Float|Clamp(Float) (.Y (Math|Vector|BreakVector _returnvalue)) -1e+03 1e+03) (.Z (Math|Vector|BreakVector _returnvalue))) false "None")))))

(event EventBeginPlay
  (CallFunction|BlendtoPlayerCamera)
  (bind _scalecurve (Timeline|ScaleUpAnim Play)
    (:Update
      (Transformation|SetRelativeScale3D (Variables|Default|GetSM_AmberBall) (Math|Conversions|ToVector(Float) _scalecurve))
      (bind _returnvalue (Utilities|Time|SetTimerbyFunctionName 0 "SpawnPlayerTrail" 0.025 true))
      (Variables|Default|SetTrailSpawnTimerHandle _returnvalue)
      (Collision|AssignOnComponentHit (Variables|Default|GetSM_AmberBall) (delegate Custom|OnComponentHit_Event_0)))))

(event Input|AxisEvents|InputAxisMoveLefRight
  (params (AxisValue :type Float%20%28single-precision%29))
  (Physics|AddForce (Variables|Default|GetSM_AmberBall) (Math|Vector|MakeVector 0.0 (* AxisValue (Variables|Default|GetHorizontalSpeedMultiplier)) 0.0) "None" false))

(fn ConstructionScript)

(fn BlendtoPlayerCamera
  (Game|Player|SetViewTargetwithBlend (Game|GetPlayerController 0) self 1.0 "VTBlend_Linear" 0.0 false))

(fn SpawnPlayerTrail
  (if (and (Variables|Default|GetbIsAlive) (not (Variables|Default|GetbHasPassed)))
    (Niagara|SpawnSystematLocation "/Game/Characters/CH01_AmberBall/NS_PlayerTrail.NS_PlayerTrail" (.location (Transformation|GetWorldTransform (Variables|Default|GetSM_AmberBall))))))

(fn HitSoundPitchManager
  (bind _returnvalue (Physics|GetPhysicsLinearVelocity (Variables|Default|GetSM_AmberBall) "None"))
  (if (>= (Math|Float|Absolute(Float) (.z _returnvalue)) 1.1e+03)
    (Audio|PlaySound2D "/Game/Sound/CharactersSounds/CHSFX00_Hit0.CHSFX00_Hit0" 1.0 1.0 0.0 0 0)
    (elif (>= (Math|Float|Absolute(Float) (.z _returnvalue)) 9e+02)
      (Audio|PlaySound2D "/Game/Sound/CharactersSounds/CHSFX01_Hit1.CHSFX01_Hit1" 1.0 1.0 0.0 0 0)
      (elif (>= (Math|Float|Absolute(Float) (.z _returnvalue)) 6e+02)
        (Audio|PlaySound2D "/Game/Sound/CharactersSounds/CHSFX02_Hit2.CHSFX02_Hit2" 1.0 1.0 0.0 0 0)
        (elif (>= (Math|Float|Absolute(Float) (.z _returnvalue)) 5e+01)
          (Audio|PlaySound2D "/Game/Sound/CharactersSounds/CHSFX03_Hit3.CHSFX03_Hit3" 1.0 1.0 0.0 0 0))))))