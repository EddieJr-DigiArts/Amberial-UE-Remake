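; BP_PlayerWinAnimation plays the AmberBall win effect on a plane, then shows the level-finished screen.
; On BeginPlay it creates a dynamic material instance and runs nested timelines for opacity, scale and Y location, each started from the previous one's Update.
; When the location timeline finishes, it adds WBP_LevelFinished to the viewport, guarded by a DoOnce flag as a workaround for repeated Finished calls.
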(event EventBeginPlay
  (bind _returnvalue (Rendering|Material|CreateDynamicMaterialInstance (Variables|Default|GetAmberballWinPlane) 0 "/Game/Characters/CH01_AmberBall/M_AmberBallWin.M_AmberBallWin" "None" :!class /Script/Engine.PrimitiveComponent))
  (bind _output_get (Variables|Default|SetMI_AmberBallWin _returnvalue))
  (bind _newtrack_0 (Timeline|OpacityAnim Play)
    (:Update
      (Rendering|Material|SetScalarParameterValue _output_get "Opacity" _newtrack_0 :!class /Script/Engine.MaterialInstanceDynamic)
      (bind _newtrack_0_2 (Timeline|ScaleAnim Play)
        (:Update
          (Transformation|SetRelativeScale3D (Variables|Default|GetAmberballWinPlane) (Math|Conversions|ToVector(Float) _newtrack_0_2))
          (bind _locationanim (Timeline|LocationAnim Play)
            (:Update
              (Transformation|SetRelativeLocation (Variables|Default|GetAmberballWinPlane) (Math|Vector|MakeVector 0.0 _locationanim 0.0) false false))
            (:Finished
              (if (not (Variables|Default|GetbDoOnce))
                (Variables|Default|SetbDoOnce true) ; Timeline Finish node is bugged, enforce do once
                (bind _returnvalue_2 (UserInterface|CreateWidget "/Game/Widgets/LevelFinish/WBP_LevelFinished.WBP_LevelFinished_C"))
                (UserInterface|Viewport|AddtoViewport _returnvalue_2 0)
                (Development|PrintString "Level Finished Widget Added by BP_WinAnimation" true true "(R=0.961658,G=0.000000,B=1.000000,A=1.000000)")))))))))

(event EventTick
  (params (DeltaSeconds :type Float%20%28single-precision%29)))

(fn ConstructionScript)