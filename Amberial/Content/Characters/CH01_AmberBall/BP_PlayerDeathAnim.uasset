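; BP_PlayerDeathAnim plays the amber ball player's death effect and then brings up the level-finished widget.
; On BeginPlay, timelines drive the broken-amber plane's opacity and scale, alongside hoop particles at the player's ball and a camera shake.
; After a one-second delay, it adds WBP_LevelFinished, guarded by a DoOnce flag.
; Tick applies radial damage around SMAmberBallDM, with the origin's X pinned to a constant.
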(event EventBeginPlay
  (Utilities|FlowControl|Sequence
    (:then_0
      (bind _returnvalue (Rendering|Material|CreateDynamicMaterialInstance (Variables|Default|GetAmberDiePlane) 0 "/Game/Characters/CH01_AmberBall/MI_AmberBallBroken.MI_AmberBallBroken" "None" :!class /Script/Engine.PrimitiveComponent))
      (bind _output_get (Variables|Default|SetMI_AmberDiePlane _returnvalue))
      (bind _newtrack_0 (Timeline|OpacityAnimation Play)
        (:Update
          (Rendering|Material|SetScalarParameterValue _output_get "OpacityStrength" _newtrack_0 :!class /Script/Engine.MaterialInstanceDynamic)
          (bind _newtrack_0_2 (Timeline|ScaleAnimation Play)
            (:Update
              (Transformation|SetRelativeScale3D (Variables|Default|GetAmberDiePlane) (Math|Conversions|ToVector(Float) _newtrack_0_2)))))))
    (:then_1
      (bind _asbp_player_character (Utilities|Casting|CastToBP_PlayerCharacter (Game|Player|GetPlayerPawn 0)))
      (Niagara|SpawnSystematLocation "/Game/Characters/CH01_AmberBall/NS_PlayerDeathHoops.NS_PlayerDeathHoops" (Transformation|GetWorldLocation (Variables|/Game/Characters/CH01_AmberBall/BP_PlayerCharacter.BP_PlayerCharacter_C|GetSM_AmberBall _asbp_player_character))))
    (:then_2
      (Game|Feedback|ClientStartCameraShake (Game|GetPlayerController 0) "/Game/Characters/CH01_AmberBall/BP_PlayerDeathCameraShake.BP_PlayerDeathCameraShake_C" 2.0 "World" "0, 0, 0")
      (Utilities|FlowControl|Delay 1.0)
      (if (not (Variables|Default|GetbDoOnce))
        (Variables|Default|SetbDoOnce true) ; Timeline Finish node is bugged, enforce do once
        (bind _returnvalue_2 (UserInterface|CreateWidget "/Game/Widgets/LevelFinish/WBP_LevelFinished.WBP_LevelFinished_C"))
        (UserInterface|Viewport|AddtoViewport _returnvalue_2 0)
        (Development|PrintString "Level Finished Widget Added by BP_Deathray" true true "(R=0.961658,G=0.000000,B=1.000000,A=1.000000)")))))

(event Collision|EventActorBeginOverlap
  (params (OtherActor :type Actor%20Object%20Reference)))

(event EventTick
  (params (DeltaSeconds :type Float%20%28single-precision%29))
  (bind _sm_amberball_dm (Variables|Default|GetSM_AmberBall_DM))
  (bind _returnvalue (Transformation|GetWorldTransform _sm_amberball_dm))
  (bind (_x _y _z) (Math|Vector|BreakVector (.location _returnvalue)))
  (Game|Damage|ApplyRadialDamage 25.0 (Math|Vector|MakeVector -15.0 _y _z) 25.0 0 0 0 0 false "ECC_Visibility"))

(fn ConstructionScript)